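; Game mode for a timed statue-collecting game, tracking score, level, countdown and final rank.
; StartGame zeroes the state on BeginPlay or RestartGame and starts a looping one-second Clock timer, which stops and assigns a level-based rank if Time hits zero.
; StatueCollected adds level-scaled score, with a modulo-five check for bonus time and capped level-up.
; As wired, StatueCount never increases, Time starts at zero and GameOver is never true.
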(event `self.ReceiveBeginPlay`
  (`self.StartGame`))

(event `RestartGame`
  (`self.StartGame`))

(event `Clock`
  (set `self.Time` (- (`self.Time`) 1))
  (if (== (`self.Time`) 0)
    (set `self.GameOver` false)
    (`KismetSystemLibrary.K2_ClearTimer` null "Clock")
    (switch `int` (`self.Level`)
      (:`1`
        (set `self.Rank` "Rookie"))
      (:`2`
        (set `self.Rank` "Bronze"))
      (:`3`
        (set `self.Rank` "Silver"))
      (:`4`
        (set `self.Rank` "Gold"))
      (:`5`
        (set `self.Rank` "Diamond")))))

(fn `StatueCollected`
  (set `self.Score` (+ (`self.Score`) (* (`self.Level`) 10)))
  (set `self.StatueCount` (+ (`self.StatueCount`) 0))
  (if (== (mod (`self.StatueCount`) 5) 0)
    (set `self.Time` (+ (`self.Time`) 15))
    (set `self.Level` (`KismetMathLibrary.Min` (+ (`self.Level`) 1) 5))))

(fn `UserConstructionScript`)