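; BP_Guide_HUD is a HUD that shows score, time and player level, plus a game-over screen.
; On BeginPlay it casts and caches the BP_Guide_GameMode.
; Each DrawHUD reads that game mode's values and draws them as colored text at fixed screen positions.
; When GameOver is set, it also draws "GAME OVER", the rank and a "Press Enter" prompt, without handling input itself.
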(event `self.ReceiveBeginPlay`
  (bind _asbp_guide_game_mode (cast `/Game/BPWeek5/Blueprints/BP_Guide_GameMode` (`GameplayStatics.GetGameMode`)))
  (set `self.My Guide Game Mode` _asbp_guide_game_mode))

(event `self.ReceiveDrawHUD`
  (params (SizeX :type Integer) (SizeY :type Integer))
  (`self.DrawText` (`KismetStringLibrary.BuildString_Int` "Score: " "" (`/Game/BPWeek5/Blueprints/BP_Guide_GameMode.Score` (`self.My Guide Game Mode`))) (struct :`R` 0.729167 :`G` 0.638235 :`B` 0.036352 :`A` 1.0) 10.0 10.0 null 3.0)
  (`self.DrawText` (`KismetStringLibrary.BuildString_Int` "Time: " "" (`/Game/BPWeek5/Blueprints/BP_Guide_GameMode.Time` (`self.My Guide Game Mode`))) (struct :`R` 0.729167 :`A` 1.0) 300.0 10.0 null 3.0)
  (`self.DrawText` (`KismetStringLibrary.BuildString_Int` "Player Level: " "" (`/Game/BPWeek5/Blueprints/BP_Guide_GameMode.Level` (`self.My Guide Game Mode`))) (struct :`G` 0.072339 :`B` 0.729167 :`A` 1.0) 550.0 10.0 null 3.0)
  (if (`/Game/BPWeek5/Blueprints/BP_Guide_GameMode.GameOver` (`self.My Guide Game Mode`))
    (`self.DrawText` "GAME OVER" (struct :`R` 0.729167 :`A` 1.0) 400.0 200.0 null 3.0)
    (`self.DrawText` "Press Enter" (struct :`R` 0.729167 :`A` 1.0) 400.0 400.0 null 3.0)
    (`self.DrawText` (`KismetStringLibrary.Concat_StrStr` "Rank: " (`/Game/BPWeek5/Blueprints/BP_Guide_GameMode.Rank` (`self.My Guide Game Mode`))) (struct :`R` 0.729167 :`A` 1.0) 400.0 300.0 null 3.0)))

(fn `UserConstructionScript`)